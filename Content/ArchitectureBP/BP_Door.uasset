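; BP_Door is a lockable door that swings open when the FirstPersonCharacter enters its Box trigger with a suitable key, and closes when they leave.
; Both overlap events pass the character's held-keys value to CanUnlock, which requires it to be evenly divisible by LockVal, so one number can satisfy several locks.
; On success, a timeline plays or reverses to drive the door's relative yaw.
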(event `self.Box.OnComponentBeginOverlap`
  (params (OverlappedComponent :type "PrimitiveComponent Object Reference") (OtherActor :type "Actor Object Reference") (OtherComp :type "PrimitiveComponent Object Reference") (OtherBodyIndex :type Integer) (bFromSweep :type Boolean) (SweepResult :type "HitResult Structure (by ref)"))
  (bind _asfirst_person_character (cast `/Game/FirstPersonBP/Blueprints/FirstPersonCharacter` OtherActor))
  (bind _keyvals (`/Game/FirstPersonBP/Blueprints/FirstPersonCharacter.GetKeysHeld` _asfirst_person_character))
  (bind _unlocks (`self.CanUnlock` _keyvals))
  (if _unlocks
    (bind (_direction _doorrotationz) (`Timeline|DoorTimelineComponent` :!label _label)
      (:`Update`
        (`SceneComponent.K2_SetRelativeRotation` (`self.Door`) (`KismetMathLibrary.MakeRotator` 0.0 0.0 _doorrotationz) false false)))))

(event `self.Box.OnComponentEndOverlap`
  (params (OverlappedComponent :type "PrimitiveComponent Object Reference") (OtherActor :type "Actor Object Reference") (OtherComp :type "PrimitiveComponent Object Reference") (OtherBodyIndex :type Integer))
  (bind _asfirst_person_character (cast `/Game/FirstPersonBP/Blueprints/FirstPersonCharacter` OtherActor))
  (bind _keyvals (`/Game/FirstPersonBP/Blueprints/FirstPersonCharacter.GetKeysHeld` _asfirst_person_character))
  (bind _unlocks (`self.CanUnlock` _keyvals))
  (if _unlocks
    (goto _label :!via `Reverse`)))

(fn `CanUnlock`
  (params (KeysHeld :type Integer))
  (returns (Unlocks :type Boolean))
  (return (== (mod KeysHeld (`self.LockVal`)) 0)))

(fn `UserConstructionScript`)